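; BP_HubCube is a StrataAR hub actor that displays an animated cube with a child BP_HubSeival and opens scene info on interaction.
; Show, run at BeginPlay, scales both meshes up from zero via a timeline, and Hide reverses it.
; Tick continuously spins both meshes and bobs them vertically with nested timelines at different rates and amplitudes.
; OnChildInteraction hides the meshes and adds a BP_SceneInfo widget to the viewport.
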(event Custom|OnChildInteraction
  (params (ID :type String))
  (switch string ID
    (:Seival
      (CallFunction|Hide)
      (bind _returnvalue (UserInterface|CreateWidget "/Game/HandheldAR/Blueprints/UI/BP_SceneInfo.BP_SceneInfo_C" (Game|GetPlayerController 0)))
      (bind _output_get (Variables|Default|SetSceneInfoWidgetRef _returnvalue))
      (UserInterface|Viewport|AddtoViewport _output_get 0))))

(event Custom|Show
  (Variables|Default|SetbActive true)
  (bind _alpha (Timeline|Timeline_1 Play)
    (:Update
      (Transformation|SetRelativeScale3D (Variables|Default|GetHubStaticMesh) (Math|Vector|MakeVector (Math|Float|Lerp 0.0 0.4 _alpha) (Math|Float|Lerp 0.0 0.4 _alpha) (Math|Float|Lerp 0.0 0.4 _alpha)))
      (Transformation|SetRelativeScale3D (Variables|/Game/StrataAR/BP_HubSeival.BP_HubSeival_C|GetStaticMesh (Variables|Default|GetSeivalHubRef)) (Math|Vector|MakeVector (Math|Float|Lerp 0.0 0.13 _alpha) (Math|Float|Lerp 0.0 0.13 _alpha) (Math|Float|Lerp 0.0 0.13 _alpha))))))

(event Custom|Hide
  (Variables|Default|SetbActive false)
  (bind _alpha (Timeline|Timeline_2 Play)
    (:Update
      (Transformation|SetRelativeScale3D (Variables|Default|GetHubStaticMesh) (Math|Vector|MakeVector (Math|Float|Lerp 0.4 0.0 _alpha) (Math|Float|Lerp 0.4 0.0 _alpha) (Math|Float|Lerp 0.4 0.0 _alpha)))
      (Transformation|SetRelativeScale3D (Variables|/Game/StrataAR/BP_HubSeival.BP_HubSeival_C|GetStaticMesh (Variables|Default|GetSeivalHubRef)) (Math|Vector|MakeVector (Math|Float|Lerp 0.13 0.0 _alpha) (Math|Float|Lerp 0.13 0.0 _alpha) (Math|Float|Lerp 0.13 0.0 _alpha))))))

(event EventBeginPlay
  (bind _returnvalue (Math|Vector|VectorZero))
  (bind _asbp_hub_seival (Utilities|Casting|CastToBP_HubSeival (Variables|/Script/Engine.ChildActorComponent|GetChildActor (Variables|Default|GetSeivalChild))))
  (Variables|Default|SetSeivalHubRef _asbp_hub_seival)
  (Transformation|SetRelativeScale3D (Variables|Default|GetHubStaticMesh) _returnvalue)
  (Transformation|SetRelativeScale3D (Variables|/Game/StrataAR/BP_HubSeival.BP_HubSeival_C|GetStaticMesh (Variables|Default|GetSeivalHubRef)) _returnvalue)
  (CallFunction|Show))

(event EventTick
  (params (DeltaSeconds :type Float%20%28single-precision%29))
  (bind _output_get (Variables|Default|SetDelta DeltaSeconds))
  (Transformation|AddLocalRotation (Variables|Default|GetHubStaticMesh) (Math|Rotator|MakeRotator 0.0 0.0 (* _output_get 25.0)) false false)
  (bind _factor (Timeline|Timeline Play)
    (:Update
      (Transformation|AddLocalOffset (Variables|Default|GetHubStaticMesh) (Math|Vector|MakeVector 0.0 0.0 (Math|Float|Lerp -0.5 0.5 _factor)) false false)
      (Transformation|AddLocalRotation (Variables|/Game/StrataAR/BP_HubSeival.BP_HubSeival_C|GetStaticMesh (Variables|Default|GetSeivalHubRef)) (Math|Rotator|MakeRotator 0.0 0.0 (* (Variables|Default|GetDelta) 15.0)) false false)
      (bind _factor_2 (Timeline|Timeline_0 Play)
        (:Update
          (Transformation|AddLocalOffset (Variables|/Game/StrataAR/BP_HubSeival.BP_HubSeival_C|GetStaticMesh (Variables|Default|GetSeivalHubRef)) (Math|Vector|MakeVector 0.0 0.0 (Math|Float|Lerp -0.2 0.2 _factor_2)) false false))))))

(fn ConstructionScript)

(fn StartCubeOffsetMovement)